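; Player gun Blueprint that handles hitscan firing, reloading from reserve ammo, a toggleable spotlight and physics-launched grenades.
; Firing checks and decrements the magazine, then line-traces from the Person_Pawn camera with random spread, applying point damage and impulses to simulated bodies.
; SpawnDecalTracer uses the trace's impact point, returned only on the physics-simulating branch, to place a bullet decal alongside a muzzle tracer.
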(event `LineTarce_Server`
  ;[1 1 1] 开火
  (bind _impactpoint (`self.LineTrace`)) ; 发射子弹轨迹函数
  (`self.SpawnDecalTracer` _impactpoint) ; 发射子弹特效和击中目标击飞并留下弹孔特效
)

(event `GunFire`
  ;[1 1 1] 开火
  (if (> (`self.CurrentAmmo`) 0)
    (`self.AmmoCheck`) ; 更新子弹数量函数
    (`self.LineTarce_Server`)
    (else
      (`GameplayStatics.PlaySoundAtLocation` "/Game/FinalGame/Sounds/DryFire.DryFire" (0.0 0.0 0.0) (struct) 1.0 1.0 0.0 null null null) ; 当前弹夹数量0，发射子弹会有空子弹的声音
    )))

(event `GunReload`
  ;[1 1 1] 装弹
  (if (and (< (`self.CurrentAmmo`) (`self.AmmoCount`)) (> (`self.TotalAmmoCount`) 0))
    (set `self.NeededAddCount` (- (`self.AmmoCount`) (`self.CurrentAmmo`))) ; 当前弹夹打出的子弹数
    (if (> (`self.NeededAddCount`) (`self.TotalAmmoCount`))
      (set `self.CurrentAmmo` (+ (`self.CurrentAmmo`) (`self.TotalAmmoCount`))) ; 当前弹夹数未补满，因为子弹不够
      (set `self.TotalAmmoCount` 0) ; 后备子弹数量为0
      (else
        (set `self.CurrentAmmo` (`self.AmmoCount`)) ; 当前弹夹数补满，因为后备子弹数够
        (set `self.TotalAmmoCount` (- (`self.TotalAmmoCount`) (`self.NeededAddCount`))) ; 更新后备子弹数
      ))
    (`GameplayStatics.PlaySoundAtLocation` "/Game/FinalGame/Sounds/Reload.Reload" (0.0 0.0 0.0) (struct) 1.0 1.0 0.0 null null null) ; 播放装弹音效
  ))

(event `GunSpotlight`
  (bind _spotlight (`self.SpotLight`))
  ;[1 1 1] 开启/关闭枪灯
  (if (`self.IsHighlight`)
    (`SceneComponent.SetVisibility` _spotlight false false)
    (set `self.IsHighlight` false)
    (else
      (`SceneComponent.SetVisibility` _spotlight true false)
      (set `self.IsHighlight` true))))

(event `GunGrenade`
  (bind _personcamera (`/Game/FinalGame/BluePrints/Person_Pawn.PersonCamera` (cast `/Game/FinalGame/BluePrints/Person_Pawn` (`GameplayStatics.GetPlayerCharacter` 0) :!pure true)))
  ;[1 1 1] 右键手雷
  (bind _returnvalue (`|SpawnActorFromClass` "/Game/FinalGame/BluePrints/Grenade/Grenade_BP.Grenade_BP_C" (`KismetMathLibrary.MakeTransform` (`SceneComponent.K2_GetComponentLocation` (`self.Muzzle`)) (`SceneComponent.K2_GetComponentRotation` _personcamera)) "Undefined" "OverrideRootScale" null null)) ; 添加手雷
  (`PrimitiveComponent.SetPhysicsLinearVelocity` (`/Game/FinalGame/BluePrints/Grenade/Grenade_BP.Grenade ` _returnvalue) (* (`SceneComponent.GetForwardVector` _personcamera) 2000.0) false "None") ; 设置手雷运动方向轨迹
)

(fn `AmmoCheck`
  ;[1 1 1] 当前弹夹内子弹数量减1，播放发射声音
  (`/Engine/EditorBlueprintResources/StandardMacros.DecrementInt` (`self.CurrentAmmo`)
    (:`  `
      (`GameplayStatics.PlaySoundAtLocation` "/Game/FinalGame/Sounds/Fire.Fire" (0.0 0.0 0.0) (struct) 1.0 1.0 0.0 null null null))))

(fn `LineTrace`
  (returns (ImpactPoint :type "Vector Structure"))
  (bind _bulletspread (`self.BulletSpread`))
  (bind _returnvalue (* _bulletspread -1.0))
  (bind _personcamera (`/Game/FinalGame/BluePrints/Person_Pawn.PersonCamera` (cast `/Game/FinalGame/BluePrints/Person_Pawn` (`GameplayStatics.GetPlayerCharacter` 0) :!pure true)))
  (set `self.WeaponHitDirection` (`KismetMathLibrary.Conv_RotatorToVector` (`SceneComponent.K2_GetComponentRotation` _personcamera))) ; 实时更新子弹方向，确保打中物体被击飞的方向
  (bind _outhit (`KismetSystemLibrary.LineTraceSingle` :`Start` (`SceneComponent.K2_GetComponentLocation` _personcamera) :`End` (+ (* (`SceneComponent.GetForwardVector` _personcamera) 200000.0) (`KismetMathLibrary.MakeVector` (`KismetMathLibrary.RandomFloatInRange` _returnvalue _bulletspread) (`KismetMathLibrary.RandomFloatInRange` _returnvalue _bulletspread) (`KismetMathLibrary.RandomFloatInRange` _returnvalue _bulletspread))) :`TraceChannel` "TraceTypeQuery2" :`DrawTime` 2.0)) ; 子弹发射轨迹
  (bind (_bblockinghit _binitialoverlap _time _distance _location _impactpoint _normal _impactnormal _physmat _hitactor _hitcomponent) (`GameplayStatics.BreakHitResult` _outhit))
  (`GameplayStatics.ApplyPointDamage` _hitactor 0.2 _impactnormal _outhit null self)
  (`KismetSystemLibrary.PrintString` (`KismetSystemLibrary.GetDisplayName` _hitactor))
  (if (`SceneComponent.IsSimulatingPhysics` _hitcomponent "None")
    (`PrimitiveComponent.AddImpulseAtLocation` _hitcomponent (* (`self.WeaponHitDirection`) (`self.WeaponDamage`)) _location "None") ; 给被子弹打中的物体力反馈效果：击飞
    (return _impactpoint) ; 用在后面给击中的物体上留下弹孔，存储弹孔的位置，注意：即使该物体没有添加力的反馈，也可以留下弹孔
  ))

(fn `SpawnDecalTracer`
  (params (`Spawn Transform Location` :type "Vector Structure"))
  (`|SpawnActorFromClass` "/Game/FinalGame/BluePrints/WeaponSpecialEffect/BulletDecal_BP.BulletDecal_BP_C" (`KismetMathLibrary.MakeTransform` `Spawn Transform Location` (`KismetMathLibrary.Conv_VectorToRotator` `Spawn Transform Location`) (0.03 0.03 0.03)) "Undefined" "OverrideRootScale" null null) ; 被子弹击中物体位置留下弹孔
  (`|SpawnActorFromClass` "/Game/FinalGame/BluePrints/WeaponSpecialEffect/MuzzleTracer_BP.MuzzleTracer_BP_C" (`KismetMathLibrary.MakeTransform` (`SceneComponent.K2_GetComponentLocation` (`self.Muzzle`)) (`SceneComponent.K2_GetComponentRotation` (`/Game/FinalGame/BluePrints/Person_Pawn.PersonCamera` (cast `/Game/FinalGame/BluePrints/Person_Pawn` (`GameplayStatics.GetPlayerCharacter` 0) :!pure true))) (0.3 0.3 0.3)) "Undefined" "OverrideRootScale" null null) ; 子弹发射时枪的火花特效
)

(fn `UserConstructionScript`
  (set `self.TotalAmmoCount` 50)
  (set `self.AmmoCount` 30)
  (set `self.CurrentAmmo` 30)
  (set `self.BulletSpread` 500.0)
  (set `self.ReloadTime` 2.0)
  (set `self.WeaponDamage` 200000.0))