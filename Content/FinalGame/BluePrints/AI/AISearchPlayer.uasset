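; AISearchPlayer is a behavior tree task that, despite its name, fires the AI's gun at the player once per execution and immediately finishes successfully.
; With ammo left, it decrements the count, plays a fire sound and traces from the gun to the player with random spread; otherwise it plays a dry-fire sound.
; The trace only draws debug, both sounds play at world origin, and the AIMoveTo branch is disconnected.
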(event `self.ReceiveExecuteAI`
  (params (OwnerController :type "AIController Object Reference") (ControlledPawn :type "Pawn Object Reference"))
  (`self.AIFire`)
  (`self.FinishExecute` true))

(event `AIFire`
  (bind _bulletspread (`self.BulletSpread`))
  (bind _returnvalue (* _bulletspread -1.0))
  (bind _aigun (`/Game/FinalGame/BluePrints/AI/AI_BP.AIGun` (cast `/Game/FinalGame/BluePrints/AI/AI_BP` (stale `self.ReceiveExecuteAI` ControlledPawn) :!pure true)))
  (bind _aicurrentammo (`/Game/FinalGame/BluePrints/AI/AIWeapon.AICurrentAmmo` _aigun))
  (if (> _aicurrentammo 0)
    (`/Engine/EditorBlueprintResources/StandardMacros.DecrementInt` _aicurrentammo
      (:`  `
        (`GameplayStatics.PlaySoundAtLocation` "/Game/FinalGame/Sounds/Fire.Fire" (0.0 0.0 0.0) (struct) 1.0 1.0 0.0 null null null)
        (`KismetSystemLibrary.LineTraceSingle` :`Start` (`SceneComponent.K2_GetComponentLocation` (`Actor.RootComponent` _aigun)) :`End` (+ (`Actor.K2_GetActorLocation` (`GameplayStatics.GetPlayerCharacter` 0)) (`KismetMathLibrary.MakeVector` (`KismetMathLibrary.RandomFloatInRange` _returnvalue _bulletspread) (`KismetMathLibrary.RandomFloatInRange` _returnvalue _bulletspread) (`KismetMathLibrary.RandomFloatInRange` _returnvalue _bulletspread))) :`TraceChannel` "TraceTypeQuery1" :`DrawDebugType` "ForDuration")))
    (else
      (`GameplayStatics.PlaySoundAtLocation` "/Game/FinalGame/Sounds/DryFire.DryFire" (0.0 0.0 0.0) (struct) 1.0 1.0 0.0 null null null))))