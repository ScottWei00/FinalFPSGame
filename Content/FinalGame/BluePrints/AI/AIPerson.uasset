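; AIPerson is the AI enemy character that shoots at its focused target, takes damage and dies.
; AIFireBullet line-traces from the weapon toward the focus actor's randomly rotated location to fake recoil, then applies point damage and plays the fire sound.
; AnyDamage lowers health and either reports a damage event for AI sensing or plays a death montage, hides the health widget and destroys the actor after a delay.
; BeginPlay links the health widget to this actor.
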(event `AIFireBullet`
  (bind _returnvalue (`AIController.GetFocusActor` (`AIBlueprintHelperLibrary.GetAIController` self)))
  ;[1 1 1] AI发射子弹
  (`/Engine/EditorBlueprintResources/StandardMacros.IsValid` _returnvalue
    (:`Is Valid`
      (bind _outhit (`KismetSystemLibrary.LineTraceSingle` (`SceneComponent.K2_GetComponentLocation` (`self.AIPersonWeaponMesh`)) (`KismetMathLibrary.GreaterGreater_VectorRotator` (`self.K2_GetActorLocation` _returnvalue) (`KismetMathLibrary.MakeRotator` (`KismetMathLibrary.RandomFloatInRange` -10.0 10.0) (`KismetMathLibrary.RandomFloatInRange` -10.0 10.0))) "TraceTypeQuery2")) ; 射线追踪，枪子弹的轨迹
      (bind (_bblockinghit _binitialoverlap _time _distance _location _impactpoint _normal _impactnormal _physmat _hitactor) (`GameplayStatics.BreakHitResult` _outhit))
      (`GameplayStatics.ApplyPointDamage` _hitactor 0.2 _impactnormal _outhit null self) ; 给被枪打到的player受到伤害
      (`GameplayStatics.PlaySoundAtLocation` "/Game/FinalGame/Sounds/Fire.Fire" (`self.K2_GetActorLocation`) (struct) 1.0 1.0 0.0 null null null) ; 播放枪发射的声音
    )))

(event `self.ReceiveAnyDamage`
  (params (Damage :type "Float (single-precision)") (DamageType :type "DamageType Object Reference") (InstigatedBy :type "Controller Object Reference") (DamageCauser :type "Actor Object Reference"))
  ;[1 1 1] AI受到伤害
  (bind _output_get (set `self.CurrentHealth` (- (`self.CurrentHealth`) Damage))) ; 每次受伤掉Damage（player发射子弹设置的是0.2）点血
  (if (<= _output_get 0.01)
    (`|PlayMontage` (`self.Mesh`) "/Game/AnimStarterPack/Death_Montage.Death_Montage" ; 播放死亡动画
      (:`then`
        (`SceneComponent.SetVisibility` (`self.HealthWidget`) false false) ; 隐藏血量text
        (`KismetSystemLibrary.Delay` 1.8) ; 死亡动画1.8秒后摧毁AI
        (`self.K2_DestroyActor`) ; 摧毁AI
      ))
    (else
      (`AISense_Damage.ReportDamageEvent` self DamageCauser Damage (`self.K2_GetActorLocation`)) ; 更新信息
    )))

(event `self.ReceiveBeginPlay`
  ;[1 1 1] 更新AI血量
  (set `/Game/FinalGame/BluePrints/AI/AIPersonHealth_HUD.Owner` self (cast `/Game/FinalGame/BluePrints/AI/AIPersonHealth_HUD` (`WidgetComponent.GetUserWidgetObject` (`self.HealthWidget`)) :!pure true)) ; 将AI的血量显示和HUD联结在一起，并实时更新
)

(fn `UserConstructionScript`)