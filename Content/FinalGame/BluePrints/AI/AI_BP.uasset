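; AI character Blueprint that carries a gun and fires debug-drawn line traces at its controller's focus actor.
; Tick prints "Hello" and fires every frame, tracing from the weapon mesh to the focus location rotated by random pitch and roll; hits are unused.
; The Construction Script attaches the weapon to the hand socket.
; Health initialization, HUD binding, damage and montage-driven death logic exist but are disconnected.
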(event `self.ReceiveBeginPlay`)

(event `self.ReceiveTick`
  (params (DeltaSeconds :type "Float (single-precision)"))
  (`KismetSystemLibrary.PrintString` "Hello")
  (`self.AIFireBullet`))

(event `AIFireBullet`
  (bind _returnvalue (`AIController.GetFocusActor` (`AIBlueprintHelperLibrary.GetAIController` self)))
  (`/Engine/EditorBlueprintResources/StandardMacros.IsValid` _returnvalue
    (:`Is Valid`
      (`KismetSystemLibrary.LineTraceSingle` :`Start` (`SceneComponent.K2_GetComponentLocation` (`self.WeaponMesh`)) :`End` (`KismetMathLibrary.GreaterGreater_VectorRotator` (`self.K2_GetActorLocation` _returnvalue) (`KismetMathLibrary.MakeRotator` (`KismetMathLibrary.RandomFloatInRange` -5.0 5.0) (`KismetMathLibrary.RandomFloatInRange` -5.0 5.0))) :`TraceChannel` "TraceTypeQuery1" :`DrawDebugType` "ForDuration" :`DrawTime` 2.0))))

(event `self.ReceiveActorBeginOverlap`
  (params (OtherActor :type "Actor Object Reference")))

(fn `UserConstructionScript`
  (`SceneComponent.K2_AttachToComponent` (`self.WeaponMesh`) (`self.Mesh`) "hand_rSocket" "KeepRelative" "KeepRelative" "KeepRelative" true) ; 在手上加把枪
)