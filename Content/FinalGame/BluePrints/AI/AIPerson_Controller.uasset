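; AI controller for person NPCs that runs the AIPerson_BT behavior tree and reacts to AI perception of the player character.
; Sensing the player writes it to the TargetActor blackboard key, sets focus on it and cancels any pending lose-target timer.
; Losing perception starts a short delay timer that then clears the blackboard target and focus, giving a grace period before the AI gives up.
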(event `self.ReceiveBeginPlay`
  (`self.RunBehaviorTree` "/Game/FinalGame/BluePrints/AI/AIPerson_BT.AIPerson_BT"))

(event `self.AIPerception.OnTargetPerceptionUpdated`
  (params (Actor :type "Actor Object Reference") (Stimulus :type "AIStimulus Structure"))
  (set `self.SensedActor` Actor) ; 将感知到的赋给变量
  (if (== Actor (`GameplayStatics.GetPlayerCharacter` 0))
    (if (`.bSuccessfullySensed` (break `AIStimulus` Stimulus))
      (`BlackboardComponent.SetValueAsObject` (`self.Blackboard`) "TargetActor" (`self.SensedActor`)) ; 传递给blackboard的变量target Actor更新为感知到的actor
      (`self.K2_SetFocus` (`self.SensedActor`)) ; 设置AI的focus为感知到的actor
      (`KismetSystemLibrary.K2_ClearAndInvalidateTimerHandle` (`self.LoseTargetTimer`))
      (else
        (bind _returnvalue (`KismetSystemLibrary.K2_SetTimerDelegate` (delegate `LoseTarget`) 3.0)) ; 感知消失执行时间
        (set `self.LoseTargetTimer` _returnvalue)))))

(event `LoseTarget`
  (`BlackboardComponent.SetValueAsObject` (`self.Blackboard`) "TargetActor" null) ; 黑板中的变量target actor更新为空
  (`self.K2_ClearFocus`) ; 清除之前的AI focus actor
)

(fn `UserConstructionScript`)