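; Networked player shooter character for an AI map and a player-versus-player map, handling movement, stance, sprint, flashlight and random replicated body color.
; Server and multicast events drive timer-repeated line-trace fire, grenades and stance flags, alongside magazine reloading.
; Authority-side damage subtracts fixed health; death shows a game-over screen against AI or restores the hidden player in place in PvP.
; Tick declares victory once no AI remain.
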(event `InputAxis|Turn`
  (params (AxisValue :type "Float (single-precision)"))
  ;[1 1 1] 鼠标控制左右转换视角
  (`self.AddControllerYawInput` AxisValue))

(event `InputAxis|MoveForward`
  (params (AxisValue :type "Float (single-precision)"))
  ;[1 1 1] 人物前后左右移动
  (`self.AddMovementInput` (`KismetMathLibrary.GetForwardVector` (`KismetMathLibrary.MakeRotator` 0.0 0.0 (.yaw (`self.GetControlRotation`)))) AxisValue))

(event `InputAxis|MoveRight`
  (params (AxisValue :type "Float (single-precision)"))
  ;[1 1 1] 人物前后左右移动
  (`self.AddMovementInput` (`KismetMathLibrary.GetRightVector` (`KismetMathLibrary.MakeRotator` 0.0 0.0 (.yaw (`self.GetControlRotation`)))) AxisValue))

(event `InputAxis|LookUp`
  (params (AxisValue :type "Float (single-precision)"))
  ;[1 1 1] 鼠标控制上下转换视角
  (`self.AddControllerPitchInput` AxisValue))

(event `BoomServer`
  ;[1 1 1] 鼠标右键手雷
  (`|SpawnActorFromClass` "/Game/FinalGame/BluePrints/Grenade/Grenade_BP.Grenade_BP_C" (`KismetMathLibrary.MakeTransform` (`SceneComponent.K2_GetComponentLocation` (`self.Muzzle`)) (`SceneComponent.K2_GetComponentRotation` (`self.PersonCamera`)) (0.3 0.3 0.3)) "Undefined" "OverrideRootScale" null null) ; 添加手雷
  (`self.BoomMulticast`) ; 手雷爆炸音效
)

(event `InputAction|Prone`
  (params (Key :type "Key Structure"))
  ;[1 1 1] Z 键卧倒和战立
  (:`Pressed`
    (`/Engine/EditorBlueprintResources/StandardMacros.FlipFlop`
      (:`A`
        (`self.Prone_Server`))
      (:`B`
        (`self.NotProne_Server`)))))

(event `InputAction|Grenade`
  (params (Key :type "Key Structure"))
  ;[1 1 1] 鼠标右键手雷
  (:`Pressed`
    (`self.boomServer`) ; 由服务器添加手雷
  ))

(event `InputAction|Crouch`
  (params (Key :type "Key Structure"))
  ;[1 1 1] C键蹲下和站立
  (:`Pressed`
    (`/Engine/EditorBlueprintResources/StandardMacros.FlipFlop` ; 按一次执行A，按另一次执行B
      (:`A`
        (`self.Crouch_Server`))
      (:`B`
        (`self.NotCrouch_Server`)))))

(event `InputAction|Jump`
  (params (Key :type "Key Structure"))
  ;[1 1 1] 空格进行人物跳跃操作
  (:`Pressed`
    (`self.Jump`))
  (:`Released`
    (`self.StopJumping`)))

(event `Prone_Server`
  ;[1 1 1] Z 键卧倒和战立
  (`self.Prone_Multicast`))

(event `Crouch_Server`
  ;[1 1 1] C键蹲下和站立
  (`self.Crouch_Multicast`))

(event `Crouch_Multicast`
  ;[1 1 1] C键蹲下和站立
  (set `self.IsCrouchPress` true))

(event `Prone_Multicast`
  ;[1 1 1] Z 键卧倒和战立
  (set `self.IsPronePress` true))

(event `BoomMulticast`
  ;[1 1 1] 鼠标右键手雷
  (`KismetSystemLibrary.Delay` 1.2) ; 手雷1.2秒后爆炸
  (`GameplayStatics.PlaySoundAtLocation` "/Game/FinalGame/Sounds/grenade.grenade" (0.0 0.0 0.0) (struct) 1.0 1.0 0.0 null null null) ; 手雷爆炸音效
)

(event `NotCrouch_Server`
  ;[1 1 1] C键蹲下和站立
  (`self.NotCrouch_Multicast`))

(event `NotCrouch_Multicast`
  ;[1 1 1] C键蹲下和站立
  (set `self.IsCrouchPress` false))

(event `NotProne_Server`
  ;[1 1 1] Z 键卧倒和战立
  (`self.NotProne_Multicast`))

(event `NotProne_Multicast`
  ;[1 1 1] Z 键卧倒和战立
  (set `self.IsPronePress` false))

(event `FireServer`
  ;[1 1 1] 鼠标左键开火，按住左键可一直开火，松开停止开火
  (bind _impactpoint (`self.WeaponLineTrace`)) ; 射线追踪，子弹会打到的位置
  (`self.WeaponSpecialEffect` _impactpoint) ; 子弹击中物体留下弹孔和发射轨迹特效
  (`self.FireMulticast`) ; 开火音效
  (`self.PlayerBulletClient`) ; 子弹更新
)

(event `Key|LeftMouseButton`
  (params (Key :type "Key Structure"))
  ;[1 1 1] 鼠标左键开火，按住左键可一直开火，松开停止开火
  (:`Pressed`
    (if (> (`self.CurrentAmmo`) 0)
      (bind _returnvalue (`KismetSystemLibrary.K2_SetTimerDelegate` (delegate `FireEvent`) 0.2 true)) ; 按住鼠标左键可连发，间隔0.2秒
      (`self.FireServer` :!label _label)
      (else
        (`self.FireClient`) ; 开火哑音
      )))
  (:`Released`
    (`KismetSystemLibrary.K2_ClearAndInvalidateTimerHandle` _returnvalue)))

(event `FireMulticast`
  ;[1 1 1] 鼠标左键开火，按住左键可一直开火，松开停止开火
  (`GameplayStatics.PlaySoundAtLocation` "/Game/FinalGame/Sounds/Fire.Fire" (`SceneComponent.K2_GetComponentLocation` (`self.Muzzle`)) (struct) 1.0 1.0 0.0 null null null) ; player开火发射子弹音效
)

(event `FireEvent`
  ;[1 1 1] 鼠标左键开火，按住左键可一直开火，松开停止开火
  (if (> (`self.CurrentAmmo`) 0)
    (goto _label)))

(event `Key|R`
  (params (Key :type "Key Structure"))
  ;[1 1 1] R键换子弹
  (:`Pressed`
    (`self.WeaponReload`) ; 武器换弹函数
  ))

(event `PlayerBulletClient`
  ;[1 1 1] 鼠标左键开火，按住左键可一直开火，松开停止开火
  (`/Engine/EditorBlueprintResources/StandardMacros.DecrementInt` (`self.CurrentAmmo`)))

(event `FireClient`
  ;[1 1 1] 鼠标左键开火，按住左键可一直开火，松开停止开火
  (`GameplayStatics.PlaySoundAtLocation` "/Game/FinalGame/Sounds/DryFire.DryFire" (`SceneComponent.K2_GetComponentLocation` (`self.Muzzle`)) (struct) 1.0 1.0 0.0 null null null) ; player开火没子弹音效
)

(event `StartSprinting`
  ;[1 1 1] 按照左Shift键可加速
  (set `CharacterMovementComponent.MaxWalkSpeed` 3000.0 (`self.CharacterMovement`)))

(event `Key|T`
  (params (Key :type "Key Structure"))
  ;[1 1 1] T键开启关闭灯光
  (:`Pressed`
    (`/Engine/EditorBlueprintResources/StandardMacros.FlipFlop`
      (:`A`
        (`self.TPressServer`))
      (:`B`
        (`self.TReleaseServer`)))))

(event `OnlyUINoGame`
  (bind _returnvalue (`GameplayStatics.GetPlayerController` 0))
  ;[1 1 1] 自定义显示UI暂停Game事件和显示game暂停UI事件
  (`WidgetBlueprintLibrary.SetInputMode_UIOnlyEx` _returnvalue null)
  (set `PlayerController.bShowMouseCursor` true _returnvalue)
  (`GameplayStatics.SetGamePaused` true))

(event `EndSprinting`
  ;[1 1 1] 按照左Shift键可加速
  (set `CharacterMovementComponent.MaxWalkSpeed` 600.0 (`self.CharacterMovement`)))

(event `TPressMulticast`
  ;[1 1 1] T键开启关闭灯光
  (`SceneComponent.SetVisibility` (`self.SpotLight`) true false))

(event `Key|LeftShift`
  (params (Key :type "Key Structure"))
  (bind _charactermovement (`self.CharacterMovement`))
  ;[1 1 1] 按照左Shift键可加速
  (:`Pressed`
    (`self.StartSprinting`)
    (set `CharacterMovementComponent.MaxWalkSpeed` 3000.0 _charactermovement))
  (:`Released`
    (`self.EndSprinting`)
    (set `CharacterMovementComponent.MaxWalkSpeed` 600.0 _charactermovement)))

(event `TPressServer`
  ;[1 1 1] T键开启关闭灯光
  (`self.TPressMulticast`))

(event `OnlyGameNoUI`
  (bind _returnvalue (`GameplayStatics.GetPlayerController` 0))
  ;[1 1 1] 自定义显示UI暂停Game事件和显示game暂停UI事件
  (`WidgetBlueprintLibrary.SetInputMode_GameOnly` _returnvalue)
  (set `PlayerController.bShowMouseCursor` false _returnvalue)
  (`GameplayStatics.SetGamePaused` false))

(event `TReleaseServer`
  ;[1 1 1] T键开启关闭灯光
  (`self.TReleaseMulticast`))

(event `TReleaseMulticast`
  ;[1 1 1] T键开启关闭灯光
  (`SceneComponent.SetVisibility` (`self.SpotLight`) false false))

(event `PlayerHurt`
  ;[1 1 1] player受到伤害，和死亡
  (bind _output_get (set `self.Health` (- (`self.Health`) 10))) ; player每次受到伤害掉10滴血
  (if (<= _output_get 0)
    (set `self.Health` 0) ; 血量为0时就不会再减少
    (bind _returnvalue (`GameplayStatics.GetCurrentLevelName` true))
    (`|ExecutionSequence`
      (:`then_0`
        (if (`KismetStringLibrary.EqualEqual_StrStr` _returnvalue "PlayerWithAI_Map")
          (`|PlayMontage` (`self.PersonMesh`) "/Game/AnimStarterPack/Death_Montage.Death_Montage" ; 播放死亡动画
            (:`then`
              (`KismetSystemLibrary.Delay` 1.8) ; 死亡动画1.8秒
              (bind _returnvalue_2 (`|CreateWidget` "/Game/FinalGame/BluePrints/HUD/PlayerWithAIDeath_HUD.PlayerWithAIDeath_HUD_C")) ; 死亡弹出本局游戏结束界面，进行操作
              (`UserWidget.AddToViewport` _returnvalue_2 0)
              (`self.OnlyUINoGame`) ; 自定义函数
            ))))
      (:`then_1`
        (if (`KismetStringLibrary.EqualEqual_StrStr` _returnvalue "PlayerWithPlayer_Map")
          (`self.Death_Server`))))))

(event `self.ReceiveAnyDamage`
  (params (Damage :type "Float (single-precision)") (DamageType :type "DamageType Object Reference") (InstigatedBy :type "Controller Object Reference") (DamageCauser :type "Actor Object Reference"))
  ;[1 1 1] player受到伤害，和死亡
  (`/Engine/EditorBlueprintResources/ActorMacros.Switch Has Authority` ; 服务器判断player是否被击中受到伤害
    (:`Authority`
      (`self.PlayerHurt`) ; 然后将伤害传给被击中的player
    )))

(event `Death_Server`
  ;[1 1 1] player受到伤害，和死亡
  (`self.Death_Multicast`))

(event `Death_Multicast`
  ;[1 1 1] player受到伤害，和死亡
  (`|PlayMontage` (`self.PersonMesh`) "/Game/AnimStarterPack/Death_Montage.Death_Montage" ; 播放死亡动画
    (:`then`
      (`KismetSystemLibrary.Delay` 1.8) ; 死亡动画1.8秒
      (`SceneComponent.SetVisibility` (`self.PersonMesh`) false false) ; 隐藏人物
      (`SceneComponent.SetVisibility` (`self.WeaponMesh`) false false) ; 隐藏枪
      (`KismetSystemLibrary.K2_SetTimerDelegate` (delegate `Reborn`) 3.0) ; 3秒后人物复活
      (`/Engine/EditorBlueprintResources/ActorMacros.Switch Has Authority`
        (:`Authority`
          (`KismetSystemLibrary.PrintString` "3秒后复活"))))))

(event `Reborn`
  ;[1 1 1] player受到伤害，和死亡
  (set `self.Health` 100)
  (set `self.CurrentAmmo` 30)
  (set `self.TotalAmmo` 230)
  (`SceneComponent.SetVisibility` (`self.PersonMesh`) true false)
  (`SceneComponent.SetVisibility` (`self.WeaponMesh`) true false))

(event `PlayerWinTheGame`
  ;[1 1 1] 击败所有AI，player获得胜利，弹出UI框
  (bind _returnvalue (`|CreateWidget` "/Game/FinalGame/BluePrints/HUD/PlayerWithAIWin_HUD.PlayerWithAIWin_HUD_C" (`GameplayStatics.GetPlayerController` 0)))
  (`UserWidget.AddToViewport` _returnvalue 0)
  (`self.OnlyUINoGame`))

(event `self.ReceiveTick`
  (params (DeltaSeconds :type "Float (single-precision)"))
  ;[1 1 1] 实时检测是否所有的AI均已被击败
  (`|ExecutionSequence`
    (:`then_0`
      (bind _returnvalue (`GameplayStatics.GetCurrentLevelName` true))
      (if (`KismetStringLibrary.EqualEqual_StrStr` _returnvalue "PlayerWithAI_Map")
        (bind _outactors (`GameplayStatics.GetAllActorsOfClass` "/Game/FinalGame/BluePrints/AI/AIPerson.AIPerson_C")) ; 获取AI这一类的所有actor
        (if (not (`KismetArrayLibrary.Array_IsValidIndex` _outactors))
          (`self.PlayerWInTheGame`))))))

(event `PersonColor`
  ;[1 1 1] 局域网人物加入和人物颜色分配
  (`/Engine/EditorBlueprintResources/ActorMacros.Switch Has Authority`
    (:`Authority`
      (`KismetSystemLibrary.PrintString` (`KismetStringLibrary.Concat_StrStr` (`KismetSystemLibrary.GetObjectName` self) " has joined") true true (struct :`G` 0.66 :`B` 1.0 :`A` 1.0) 3.0) ; 每有一个人加入则在服务端显示人物加入
      (set `self.Color` (make `LinearColor` (`KismetMathLibrary.RandomFloatInRange` 0.0 1.0) (`KismetMathLibrary.RandomFloatInRange` 0.0 1.0) (`KismetMathLibrary.RandomFloatInRange` 0.0 1.0) 1.0)) ; 给每个局域网内的人物添加随机颜色
    )))

(event `self.ReceiveBeginPlay`
  ;[1 1 1] player加入时随机分配颜色
  (`|ExecutionSequence`
    (:`then_0`
      (`self.PersonColor`) ; 设置人物皮肤颜色
    )
    (:`then_1`
      (`LightComponent.SetLightColor` (`self.SpotLight`) (`self.Color`) true) ; 设置聚光灯的颜色和人物皮肤颜色相同
    )))

(fn `OnRep_Color`
  (bind _returnvalue (`PrimitiveComponent.CreateDynamicMaterialInstance` (`self.PersonMesh`) 0 "/Game/AnimStarterPack/UE4_Mannequin/Materials/M_UE4Man_Body.M_UE4Man_Body" "None")) ; 人物更换颜色
  (`MaterialInstanceDynamic.SetVectorParameterValue` _returnvalue "BodyColor" (`self.Color`)) ; 设置颜色
)

(fn `OnRep_IsSpotlightVisible`)

(fn `UserConstructionScript`)

(fn `WeaponLineTrace`
  (returns (ImpactPoint :type "Vector Structure"))
  (bind _personcamera (`self.PersonCamera`))
  ;[1 1 1] 发射子弹的轨迹以及力反馈效果
  (set `self.WeaponHitDirection` (`KismetMathLibrary.Conv_RotatorToVector` (`SceneComponent.K2_GetComponentRotation` _personcamera))) ; 击中物体产生力作用的方向
  (bind _outhit (`KismetSystemLibrary.LineTraceSingle` (`SceneComponent.K2_GetComponentLocation` _personcamera) (* (`SceneComponent.GetForwardVector` _personcamera) 200000.0) "TraceTypeQuery2")) ; 子弹发射轨迹
  (bind (_bblockinghit _binitialoverlap _time _distance _location _impactpoint _normal _impactnormal _physmat _hitactor _hitcomponent) (`GameplayStatics.BreakHitResult` _outhit))
  (set `self.Hit Component` _hitcomponent)
  (`GameplayStatics.ApplyPointDamage` _hitactor 0.2 _impactnormal _outhit null self) ; 子弹击中人受到的伤害
  (if (`SceneComponent.IsSimulatingPhysics` (`self.Hit Component`) "None")
    (`PrimitiveComponent.AddImpulseAtLocation` (`self.Hit Component`) (* (`self.WeaponHitDirection`) (`self.WeaponDamage`)) _location "None") ; 添加力反馈
  )
  (return _impactpoint) ; 将击中位置返回在后面进行加入特效
)

(fn `WeaponReload`
  ;[1 1 1] 换弹操作
  (if (and (< (`self.CurrentAmmo`) (`self.MaxAmmo`)) (> (`self.TotalAmmo`) 0))
    (`GameplayStatics.PlaySoundAtLocation` "/Game/FinalGame/Sounds/Reload.Reload" (0.0 0.0 0.0) (struct) 1.0 1.0 0.0 null null null) ; 播放换弹音效
    (set `self.NeededAddBullet` (- (`self.MaxAmmo`) (`self.CurrentAmmo`))) ; 当前弹夹需要补充的子弹数
    (if (> (`self.NeededAddBullet`) (`self.TotalAmmo`))
      (set `self.CurrentAmmo` (+ (`self.CurrentAmmo`) (`self.TotalAmmo`)))
      (set `self.TotalAmmo` 0)
      (else
        (set `self.CurrentAmmo` (`self.MaxAmmo`))
        (set `self.TotalAmmo` (- (`self.TotalAmmo`) (`self.NeededAddBullet`)))))))

(fn `WeaponSpecialEffect`
  (params (SpawnTransform_Location :type "Vector Structure"))
  ;[1 1 1] 开火特效：击中物体时留下弹孔和子弹发射轨迹特效
  (`|SpawnActorFromClass` "/Game/FinalGame/BluePrints/WeaponSpecialEffect/BulletDecal_BP.BulletDecal_BP_C" (`KismetMathLibrary.MakeTransform` SpawnTransform_Location (`KismetMathLibrary.Conv_VectorToRotator` SpawnTransform_Location) (0.1 0.1 0.1)) "Undefined" "OverrideRootScale" null null) ; 击中物体时会留下弹孔，3秒后弹孔自动消失
  (`|SpawnActorFromClass` "/Game/FinalGame/BluePrints/WeaponSpecialEffect/MuzzleTracer_BP.MuzzleTracer_BP_C" (`KismetMathLibrary.MakeTransform` (`SceneComponent.K2_GetComponentLocation` (`self.Muzzle`)) (`SceneComponent.K2_GetComponentRotation` (`self.PersonCamera`)) (0.3 0.3 0.3)) "Undefined" "OverrideRootScale" null null) ; 发射子弹会有子弹发射特效
)