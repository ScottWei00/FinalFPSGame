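; Behavior tree service that lets an AI person shoot at its focus actor when it has a clear line to it.
; On activation it caches the controller and the pawn cast to AIPerson.
; Each tick it sphere-traces on the Camera channel from the pawn to the focus actor, ignoring itself.
; If the trace hits that focus actor first, it calls AIFireBullet on the pawn.
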(event `self.ReceiveActivationAI`
  (params (OwnerController :type "AIController Object Reference") (ControlledPawn :type "Pawn Object Reference"))
  (set `self.Owner Controller` OwnerController)
  (bind _asaiperson (cast `/Game/FinalGame/BluePrints/AIIIIIIII/AIPerson` ControlledPawn))
  (set `self.As AIPerson` _asaiperson))

(event `self.ReceiveTickAI`
  (params (OwnerController :type "AIController Object Reference") (ControlledPawn :type "Pawn Object Reference") (DeltaSeconds :type "Float (single-precision)"))
  (bind (_outhit _returnvalue) (`KismetSystemLibrary.SphereTraceSingle` (`Actor.K2_GetActorLocation` ControlledPawn) (`Actor.K2_GetActorLocation` (`AIController.GetFocusActor` OwnerController)) 64.0 "TraceTypeQuery2" false (`|MakeArray` (`self.As AIPerson`) :!type "Actor Object Reference")))
  (if _returnvalue
    (if (== (`.HitActor` (`GameplayStatics.BreakHitResult` _outhit)) (`AIController.GetFocusActor` (`self.Owner Controller`)))
      (`/Game/FinalGame/BluePrints/AIIIIIIII/AIPerson.AIFireBullet` (`self.As AIPerson`)))))