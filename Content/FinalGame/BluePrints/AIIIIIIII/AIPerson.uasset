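; AI-controlled armed character that fires hitscan shots and dies when its health runs out.
; AIFireBullet traces on the Camera channel from the weapon mesh toward the controller's focus actor, applies point damage and plays a fire sound.
; Spread comes from randomly rotating the target's world position vector, so it scales with distance from the world origin.
; AnyDamage lowers health, then destroys the actor or reports a damage event to AI perception.
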(event `AIFireBullet`
  (bind _returnvalue (`AIController.GetFocusActor` (`AIBlueprintHelperLibrary.GetAIController` self)))
  (`/Engine/EditorBlueprintResources/StandardMacros.IsValid` _returnvalue
    (:`Is Valid`
      (bind _outhit (`KismetSystemLibrary.LineTraceSingle` :`Start` (`SceneComponent.K2_GetComponentLocation` (`self.AIPersonWeaponMesh`)) :`End` (`KismetMathLibrary.GreaterGreater_VectorRotator` (`self.K2_GetActorLocation` _returnvalue) (`KismetMathLibrary.MakeRotator` (`KismetMathLibrary.RandomFloatInRange` -10.0 10.0) (`KismetMathLibrary.RandomFloatInRange` -10.0 10.0))) :`TraceChannel` "TraceTypeQuery2" :`DrawDebugType` "ForDuration"))
      (bind (_bblockinghit _binitialoverlap _time _distance _location _impactpoint _normal _impactnormal _physmat _hitactor) (`GameplayStatics.BreakHitResult` _outhit))
      (`GameplayStatics.ApplyPointDamage` _hitactor 0.2 _impactnormal _outhit null self)
      (`GameplayStatics.PlaySoundAtLocation` "/Game/FinalGame/Sounds/Fire.Fire" (`self.K2_GetActorLocation`) (struct) 1.0 1.0 0.0 null null null))))

(event `self.ReceiveAnyDamage`
  (params (Damage :type "Float (single-precision)") (DamageType :type "DamageType Object Reference") (InstigatedBy :type "Controller Object Reference") (DamageCauser :type "Actor Object Reference"))
  (bind _currenthealth (`self.CurrentHealth`))
  (bind _output_get (set `self.CurrentHealth` (- _currenthealth Damage)))
  (`KismetSystemLibrary.PrintString` (`KismetStringLibrary.Conv_DoubleToString` _currenthealth))
  (if (<= _output_get 0.0)
    (`self.K2_DestroyActor`)
    (else
      (`AISense_Damage.ReportDamageEvent` self DamageCauser Damage (`self.K2_GetActorLocation`)))))

(fn `UserConstructionScript`)